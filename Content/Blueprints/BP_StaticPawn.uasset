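; BP_StaticPawn is a player pawn that pans a camera within fixed bounds and tracks the currently selected character.
; Axis inputs offset the actor's X and Y location by CameraSpeed, clamped to hard-coded limits and not scaled by delta time.
; SelectCharacter deselects any previous character before storing and selecting the new one.
; Holding Tab triggers hover messages on every BPI_Interactable actor, and releasing it ends them.
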(event `Select Character`
  (params (`Character To Select` :type "/Game/Blueprints/BP_Character Object Reference"))
  ;[1 1 1] Character Selection
  (`self.Deselect Character`)
  (bind _output_get (set `self.SelectedCharacter` `Character To Select`))
  (`/Game/Blueprints/BP_Character.Select` _output_get))

(event `Deselect Character`
  (bind _selectedcharacter (`self.SelectedCharacter`))
  ;[1 1 1] Character Selection
  (`/Engine/EditorBlueprintResources/StandardMacros.IsValid` _selectedcharacter
    (:`Is Valid`
      (`/Game/Blueprints/BP_Character.Deselect` _selectedcharacter)
      (set `self.SelectedCharacter` null))))

(event `InputAxis|HorizontalAxis`
  (params (AxisValue :type "Float (single-precision)"))
  (bind (_returnvalue_x _returnvalue_y _returnvalue_z) (`KismetMathLibrary.BreakVector` (`self.K2_GetActorLocation`)))
  ;[1 1 1] Camera Movement
  (`self.K2_SetActorLocation` (`KismetMathLibrary.MakeVector` _returnvalue_x (`KismetMathLibrary.FClamp` (+ (* (`self.CameraSpeed`) AxisValue) _returnvalue_y) -200.0 800.0) _returnvalue_z)))

(event `InputAxis|ForwardAxis`
  (params (AxisValue :type "Float (single-precision)"))
  (bind (_returnvalue_x _returnvalue_y _returnvalue_z) (`KismetMathLibrary.BreakVector` (`self.K2_GetActorLocation`)))
  ;[1 1 1] Camera Movement
  (`self.K2_SetActorLocation` (`KismetMathLibrary.MakeVector` (`KismetMathLibrary.FClamp` (+ _returnvalue_x (* (`self.CameraSpeed`) AxisValue)) -1000.0 -300.0) _returnvalue_y _returnvalue_z)))

(event `Key|Tab`
  (params (Key :type "Key Structure"))
  (:`Pressed`
    (bind _outactors (`GameplayStatics.GetAllActorsWithInterface` "/Game/Blueprints/BPI_Interactable.BPI_Interactable_C"))
    (for _array_element _outactors
      (message `/Game/Blueprints/BPI_Interactable.OnHover` _array_element)))
  (:`Released`
    (bind _outactors_2 (`GameplayStatics.GetAllActorsWithInterface` "/Game/Blueprints/BPI_Interactable.BPI_Interactable_C"))
    (for _array_element_2 _outactors_2
      (message `/Game/Blueprints/BPI_Interactable.OnHoverEnd` _array_element_2))))

(fn `UserConstructionScript`)