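; BP_CharacterSlot is a clickable slot where the player places the character currently selected in BP_StaticPawn.
; Clicking a free slot teleports that character to the slot, deselects it and marks the slot occupied.
; Clicking an occupied slot rechecks for overlapping BP_Character actors and frees it if none remain, a self-admitted hack, before placing.
; Cursor hover toggles a Highlight material parameter on the slot visual.
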(event `self.Slot.OnClicked`
  (params (TouchedComponent :type "PrimitiveComponent Object Reference") (ButtonPressed :type "Key Structure"))
  (if (`self.bIsFree`)
    (bind _asbp_static_pawn (cast `/Game/Game/BP_StaticPawn` (`GameplayStatics.GetPlayerPawn` 0) :!label _label))
    (bind _selectedcharacter (`/Game/Game/BP_StaticPawn.SelectedCharacter` _asbp_static_pawn))
    (`/Engine/EditorBlueprintResources/StandardMacros.IsValid` _selectedcharacter
      (:`Is Valid`
        (`self.K2_SetActorLocation` _selectedcharacter (`self.K2_GetActorLocation`) false true)
        (`/Game/Game/BP_StaticPawn.Deselect Character` _asbp_static_pawn)
        (set `self.bIsFree` false)))
    (else
      ;[1 1 1] That is a very bad hack :)
      (bind _output_get (`self.Check If Character Is In Slot`))
      (if _output_get
        (goto _label)))))

(event `self.Slot.OnBeginCursorOver`
  (params (TouchedComponent :type "PrimitiveComponent Object Reference"))
  (`self.OnHover`))

(event `self.Slot.OnEndCursorOver`
  (params (TouchedComponent :type "PrimitiveComponent Object Reference"))
  (`self.OnHoverEnd`))

(fn `Check If Character Is In Slot`
  (returns (Output_Get :type Boolean))
  (if (== (`KismetArrayLibrary.Array_Length` (`PrimitiveComponent.GetOverlappingActors` (`self.Slot`) "/Game/Blueprints/BP_Character.BP_Character_C")) 0)
    (bind _output_get (set `self.bIsFree` true))
    (return _output_get)))

(fn `OnHover`
  (`MeshComponent.SetScalarParameterValueOnMaterials` (`self.SlotVisual`) "Highlight" 0.01))

(fn `OnHoverEnd`
  (`MeshComponent.SetScalarParameterValueOnMaterials` (`self.SlotVisual`) "Highlight" 0.0))

(fn `UserConstructionScript`)