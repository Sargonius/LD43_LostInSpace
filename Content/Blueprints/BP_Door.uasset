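; BP_Door is a clickable door that slides along its local Z axis to open and close.
; Clicking DoorMesh alternates Open and Close through a FlipFlop and records the state in IsOpen.
; The DoorInteraction timeline drives DoorPivot's relative Z from DoorOffset, playing to open and reversing to close.
; Cursor hover toggles a Highlight scalar parameter on the mesh materials.
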(event `Open`
  (bind (_direction _door_offset) (`Timeline|Door Interaction` :!label _label)
    (:`Update`
      (`SceneComponent.K2_SetRelativeLocation` (`self.DoorPivot`) (`KismetMathLibrary.MakeVector` 0.0 0.0 _door_offset) false false))))

(event `Close`
  (goto _label :!via `Reverse`))

(event `self.DoorMesh.OnClicked`
  (params (TouchedComponent :type "PrimitiveComponent Object Reference") (ButtonPressed :type "Key Structure"))
  (`self.OnClick`))

(event `self.DoorMesh.OnBeginCursorOver`
  (params (TouchedComponent :type "PrimitiveComponent Object Reference"))
  (`self.OnHover`))

(event `self.OnClick`
  (`/Engine/EditorBlueprintResources/StandardMacros.FlipFlop`
    (:`A`
      (`self.Open`)
      (set `self.bIsOpen` true))
    (:`B`
      (`self.Close`)
      (set `self.bIsOpen` false))))

(event `self.DoorMesh.OnEndCursorOver`
  (params (TouchedComponent :type "PrimitiveComponent Object Reference"))
  (`self.OnHoverEnd`))

(fn `OnHover`
  (`MeshComponent.SetScalarParameterValueOnMaterials` (`self.DoorMesh`) "Highlight" 1.0))

(fn `OnHoverEnd`
  (`MeshComponent.SetScalarParameterValueOnMaterials` (`self.DoorMesh`) "Highlight" 0.0))

(fn `UserConstructionScript`)