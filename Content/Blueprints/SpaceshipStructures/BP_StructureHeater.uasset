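; Clickable spaceship heater structure that the player toggles on and off, starting deactivated at BeginPlay.
; Clicks on the Heater component call Activate or Deactivate on top of parent logic, with activation feedback shown only when fuel remains.
; State changes drive a material Highlight parameter, two power indicator materials and a sound.
; Cursor hover adds to the stored highlight level, so hover and powered glow stack.
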(event `self.ReceiveBeginPlay`
  (`parent.ReceiveBeginPlay`)
  (`self.Deactivate`))

(event `self.Activate`
  (`parent.Activate`)
  (if (> (`/Game/Blueprints/BPF_LostInSpace.Get Fuel`) 0.0)
    (set `self.CurrentHighlight` 1.0)
    (`MeshComponent.SetScalarParameterValueOnMaterials` (`self.Heater`) "Highlight" (`self.CurrentHighlight`))
    (`PrimitiveComponent.SetMaterial` (`self.Indicator`) 0 "/Game/Materials/MI_PowerIndicator_On.MI_PowerIndicator_On")
    (`PrimitiveComponent.SetMaterial` (`self.Indicator2`) 0 "/Game/Materials/MI_PowerIndicator_On.MI_PowerIndicator_On")
    (`GameplayStatics.PlaySoundAtLocation` "/Game/Sounds/S_EnableHeater.S_EnableHeater" (`self.K2_GetActorLocation`) (struct) 0.45 1.0 0.0 null null null)))

(event `self.Heater.OnBeginCursorOver`
  (params (TouchedComponent :type "PrimitiveComponent Object Reference"))
  (`self.OnHover`))

(event `self.Deactivate`
  (`parent.Deactivate`)
  (set `self.CurrentHighlight` 0.0)
  (`MeshComponent.SetScalarParameterValueOnMaterials` (`self.Heater`) "Highlight" (`self.CurrentHighlight`))
  (`PrimitiveComponent.SetMaterial` (`self.Indicator`) 0 "/Game/Materials/MI_PowerIndicator_Off.MI_PowerIndicator_Off")
  (`PrimitiveComponent.SetMaterial` (`self.Indicator2`) 0 "/Game/Materials/MI_PowerIndicator_Off.MI_PowerIndicator_Off")
  (`GameplayStatics.PlaySoundAtLocation` "/Game/Sounds/S_Deactivate.S_Deactivate" (`self.K2_GetActorLocation`) (struct) 0.5 1.0 0.0 null null null))

(event `self.Heater.OnEndCursorOver`
  (params (TouchedComponent :type "PrimitiveComponent Object Reference"))
  (`self.OnHoverEnd`))

(event `self.OnClick`
  (if (`self.bIsEnabled`)
    (`self.Deactivate`)
    (else
      (`self.Activate`))))

(event `self.Heater.OnClicked`
  (params (TouchedComponent :type "PrimitiveComponent Object Reference") (ButtonPressed :type "Key Structure"))
  (`self.OnClick`))

(fn `OnHover`
  (`parent.OnHover`)
  (`MeshComponent.SetScalarParameterValueOnMaterials` (`self.Heater`) "Highlight" (+ (`self.CurrentHighlight`) 1.0)))

(fn `OnHoverEnd`
  (`parent.OnHoverEnd`)
  (`MeshComponent.SetScalarParameterValueOnMaterials` (`self.Heater`) "Highlight" (+ (`self.CurrentHighlight`) 0.0)))

(fn `UserConstructionScript`
  (`parent.UserConstructionScript`))