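; Spaceship oxygen generator structure that the player toggles on and off by clicking its cylinder mesh.
; It starts deactivated, and activation or deactivation extends the parent behavior by switching the oxygen VFX and swapping the power indicator material.
; Cursor hover on the cylinder sets a Highlight material parameter for visual feedback.
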(event `self.ReceiveBeginPlay`
  (`parent.ReceiveBeginPlay`)
  (`self.Deactivate`))

(event `self.Activate`
  (`parent.Activate`)
  (`ActorComponent.Activate` (`self.OxygenVFX`) true)
  (`PrimitiveComponent.SetMaterial` (`self.EnabledIndicator`) 0 "/Game/Materials/MI_PowerIndicator_On.MI_PowerIndicator_On"))

(event `self.Deactivate`
  (`parent.Deactivate`)
  (`ActorComponent.Deactivate` (`self.OxygenVFX`))
  (`PrimitiveComponent.SetMaterial` (`self.EnabledIndicator`) 0 "/Game/Materials/MI_PowerIndicator_Off.MI_PowerIndicator_Off"))

(event `self.Cylinder.OnClicked`
  (params (TouchedComponent :type "PrimitiveComponent Object Reference") (ButtonPressed :type "Key Structure"))
  (`self.OnClick`))

(event `self.OnClick`
  (if (`self.bIsEnabled`)
    (`self.Deactivate`)
    (else
      (`self.Activate`))))

(event `self.Cylinder.OnBeginCursorOver`
  (params (TouchedComponent :type "PrimitiveComponent Object Reference"))
  (`self.OnHover`))

(event `self.Cylinder.OnEndCursorOver`
  (params (TouchedComponent :type "PrimitiveComponent Object Reference"))
  (`self.OnHoverEnd`))

(fn `OnHover`
  (`MeshComponent.SetScalarParameterValueOnMaterials` (`self.Cylinder`) "Highlight" 1.0))

(fn `OnHoverEnd`
  (`MeshComponent.SetScalarParameterValueOnMaterials` (`self.Cylinder`) "Highlight" 0.0))

(fn `UserConstructionScript`)