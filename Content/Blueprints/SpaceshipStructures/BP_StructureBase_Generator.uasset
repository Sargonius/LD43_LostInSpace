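; A clickable power generator structure for the spaceship that starts switched off on BeginPlay.
; Clicking the generator mesh toggles it between Activate and Deactivate, which extend the parent's logic by setting the room light intensity, the light's glow and the indicator's on/off material.
; Cursor hover events on the generator mesh call overridden hover functions that drive its Highlight material parameter.
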(event `self.Activate`
  (`parent.Activate`)
  (`LightComponent.SetIntensity` (`self.RoomLight`) 5000.0)
  (`MeshComponent.SetScalarParameterValueOnMaterials` (`self.Light`) "Highlight" 3.0)
  (`PrimitiveComponent.SetMaterial` (`self.Indicator`) 0 "/Game/Materials/MI_PowerIndicator_On.MI_PowerIndicator_On"))

(event `self.Deactivate`
  (`parent.Deactivate`)
  (`LightComponent.SetIntensity` (`self.RoomLight`) 0.0)
  (`MeshComponent.SetScalarParameterValueOnMaterials` (`self.Light`) "Highlight" 0.0)
  (`PrimitiveComponent.SetMaterial` (`self.Indicator`) 0 "/Game/Materials/MI_PowerIndicator_Off.MI_PowerIndicator_Off"))

(event `self.OnClick`
  (if (`self.bIsEnabled`)
    (`self.Deactivate`)
    (else
      (`self.Activate`))))

(event `self.ReceiveBeginPlay`
  (`parent.ReceiveBeginPlay`)
  (`self.Deactivate`))

(event `self.PowerGenerator.OnClicked`
  (params (TouchedComponent :type "PrimitiveComponent Object Reference") (ButtonPressed :type "Key Structure"))
  (`self.OnClick`))

(event `self.PowerGenerator.OnBeginCursorOver`
  (params (TouchedComponent :type "PrimitiveComponent Object Reference"))
  (`self.OnHover`))

(event `self.PowerGenerator.OnEndCursorOver`
  (params (TouchedComponent :type "PrimitiveComponent Object Reference"))
  (`self.OnHoverEnd`))

(fn `OnHover`
  (`parent.OnHover`)
  (`MeshComponent.SetScalarParameterValueOnMaterials` (`self.PowerGenerator`) "Highlight" 1.0))

(fn `OnHoverEnd`
  (`parent.OnHoverEnd`)
  (`MeshComponent.SetScalarParameterValueOnMaterials` (`self.PowerGenerator`) "Highlight" 0.0))

(fn `UserConstructionScript`
  (`parent.UserConstructionScript`))