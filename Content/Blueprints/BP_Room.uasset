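; Room actor that simulates heat, oxygen and power, plus decompression that switches off gravity for characters inside.
; A one-second timer raises or drains each clamped resource based on its machine's enabled state, though Heat and Power ignore the passed amount and step by one.
; A second timer marks the room decompressed only when all monitored doors are open, then updates gravity on overlapping characters' bodies.
; An info widget receives a room reference.
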(event `Room Resource Tick`
  (`|ExecutionSequence`
    (:`then_0`
      (if (`/Game/Blueprints/SpaceshipStructures/BP_StructureBase.bIsEnabled` (`self.Heater`))
        (`self.Add Resource` "NewEnumerator1" 4.0)
        (else
          (`self.Consume Resource` "NewEnumerator1" 1.5))))
    (:`then_1`
      (if (`/Game/Blueprints/SpaceshipStructures/BP_StructureBase.bIsEnabled` (`self.OxygenGenerator`))
        (`self.Add Resource` "NewEnumerator0" 4.0)
        (else
          (`self.Consume Resource` "NewEnumerator0" 0.5))))
    (:`then_2`
      (if (`/Game/Blueprints/SpaceshipStructures/BP_StructureBase.bIsEnabled` (`self.Generator`))
        (`self.Add Resource` "NewEnumerator2" 4.0)
        (else
          (`self.Consume Resource` "NewEnumerator2" 2.5))))))

(event `self.ReceiveBeginPlay`
  (bind _aswbp_room_info (cast `/Game/Widgets/WBP_RoomInfo` (`WidgetComponent.GetUserWidgetObject` (`self.InfoWidget`))))
  (set `/Game/Widgets/WBP_RoomInfo.RoomReference` self _aswbp_room_info)
  (`KismetSystemLibrary.K2_SetTimerDelegate` (delegate `Check For Pressure`) 1.0 true)
  (`KismetSystemLibrary.K2_SetTimerDelegate` (delegate `Room Resource Tick`) 1.0 true))

(event `Toggle Gravity`
  (for _array_element (`PrimitiveComponent.GetOverlappingActors` (`self.Room`) "/Game/Blueprints/BP_Character.BP_Character_C")
    (bind _asbp_character (cast `/Game/Blueprints/BP_Character` _array_element))
    (bind _characterbody (`/Game/Blueprints/BP_Character.CharacterBody` _asbp_character))
    (`/Engine/EditorBlueprintResources/StandardMacros.IsValid` _characterbody
      (:`Is Valid`
        (`PrimitiveComponent.SetEnableGravity` _characterbody (not (`self.bIsDecompressed`)))))))

(event `Check For Pressure`
  (set `self.bDecompressionCheck` false)
  (for _array_element (`self.DoorsToCheckForPressure`)
    (if (not (`/Game/Blueprints/BP_Door.bIsOpen` _array_element))
      (set `self.bDecompressionCheck` true)))
  (set `self.bIsDecompressed` (not (`self.bDecompressionCheck`)))
  (`self.Toggle Gravity`))

(fn `Add Resource`
  (params (Resource :type "/Game/Blueprints/EResource Enum" :default "NewEnumerator0") (Amount :type "Float (double-precision)"))
  (switch `/Game/Blueprints/EResource` Resource
    (:`NewEnumerator0`
      (set `self.Oxygen` (`KismetMathLibrary.FClamp` (+ (`self.Oxygen`) Amount) 0.0 100.0)))
    (:`NewEnumerator1`
      (set `self.Heat` (`KismetMathLibrary.FClamp` (+ (`self.Heat`) 1.0) 0.0 100.0)))
    (:`NewEnumerator2`
      (set `self.Power` (`KismetMathLibrary.FClamp` (+ (`self.Power`) 1.0) 0.0 100.0)))))

(fn `Consume Resource`
  (params (Resource :type "/Game/Blueprints/EResource Enum" :default "NewEnumerator0") (Amount :type "Float (double-precision)"))
  (switch `/Game/Blueprints/EResource` Resource
    (:`NewEnumerator0`
      (set `self.Oxygen` (`KismetMathLibrary.FClamp` (- (`self.Oxygen`) Amount) 0.0 100.0)))
    (:`NewEnumerator1`
      (set `self.Heat` (`KismetMathLibrary.FClamp` (- (`self.Heat`) 1.0) 0.0 100.0)))
    (:`NewEnumerator2`
      (set `self.Power` (`KismetMathLibrary.FClamp` (- (`self.Power`) 1.0) 0.0 100.0)))))

(fn `UserConstructionScript`)