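; Selectable cube character with randomized oxygen, heat and power needs, drawn from the BP_Room it last overlapped.
; A looping randomized timer consumes those resources or drains Health when they run low; death decrements SavedCubes in the game instance.
; Clicks toggle selection through BP_StaticPawn while gravity is enabled, and a status widget displays speech.
; A self-restarting timeline blinks the eyes, and a separate event hides the cube with an explosion effect.
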(event `self.ReceiveBeginPlay`
  (`self.Blink`)
  (`ActorComponent.Deactivate` (`self.CharacterSelectionEffect`))
  (`KismetSystemLibrary.K2_SetTimerDelegate` (delegate `Needs Tick`) (`KismetMathLibrary.RandomFloatInRange` 0.8 2.5) true)
  (`self.Generate Cube Parameters`)
  ;[1 1 1] Cube ref in needs widget
  (bind _aswbp_character_status (cast `/Game/Widgets/WBP_CharacterStatus` (`WidgetComponent.GetUserWidgetObject` (`self.CharacterStatusWidget`))))
  (`/Game/Widgets/WBP_CharacterStatus.Set Cube Reference` _aswbp_character_status self))

(event `Key|Shift+K` :consume false :overrideparent false
  (params (Key :type "Key Structure"))
  ;[1 0 0] DEBUG Kill all cubes
  (:`Pressed`
    (`self.Death`)))

(event `self.OnClick`
  ;[1 1 1] Cube selection-deselection
  (if (`PrimitiveComponent.IsGravityEnabled` (`self.CharacterBody`))
    (bind _asbp_static_pawn (cast `/Game/Blueprints/BP_StaticPawn` (`GameplayStatics.GetPlayerPawn` 0)))
    (if (== (`/Game/Blueprints/BP_StaticPawn.SelectedCharacter` _asbp_static_pawn) self)
      (`/Game/Blueprints/BP_StaticPawn.Deselect Character` _asbp_static_pawn)
      (else
        (`/Game/Blueprints/BP_StaticPawn.Select Character` _asbp_static_pawn self)))))

(event `self.CharacterBody.OnBeginCursorOver`
  (params (TouchedComponent :type "PrimitiveComponent Object Reference"))
  ;[1 1 1] Hover
  (`self.OnHover`))

(event `self.CharacterBody.OnComponentBeginOverlap`
  (params (OverlappedComponent :type "PrimitiveComponent Object Reference") (OtherActor :type "Actor Object Reference") (OtherComp :type "PrimitiveComponent Object Reference") (OtherBodyIndex :type Integer) (bFromSweep :type Boolean) (SweepResult :type "HitResult Structure (by ref)"))
  ;[1 1 1] Cube is in new room
  (if (`self.bIsAlive`)
    (bind _asbp_room (cast `/Game/Blueprints/BP_Room` OtherActor))
    (set `self.RoomReference` _asbp_room)
    (if (`KismetMathLibrary.RandomBool`)
      (`self.Say` "This room is nice!")
      (elif (`KismetMathLibrary.RandomBool`)
        (`self.Say` "Weeee!")))))

(event `self.CharacterBody.OnEndCursorOver`
  (params (TouchedComponent :type "PrimitiveComponent Object Reference"))
  ;[1 1 1] Hover
  (`self.OnHoverEnd`))

(event `Needs Tick`
  (bind _roomreference (`self.RoomReference`))
  ;[1 1 1] Needs
  (`/Engine/EditorBlueprintResources/StandardMacros.IsValid` _roomreference
    (:`Is Valid`
      (if (`self.bIsAlive`)
        (`|ExecutionSequence`
          (:`then_0`
            (if (> (`/Game/Blueprints/BP_Room.Oxygen` _roomreference) 1.0)
              (`/Game/Blueprints/BP_Room.Consume Resource` (`self.RoomReference`) "NewEnumerator0" (`self.Lungs`))
              (else
                (set `self.Health` (- (`self.Health`) (`KismetMathLibrary.RandomFloatInRange` 0.8 1.3)) :!label _label))))
          (:`then_1`
            (if (> (`/Game/Blueprints/BP_Room.Heat` _roomreference) 1.0)
              (`/Game/Blueprints/BP_Room.Consume Resource` (`self.RoomReference`) "NewEnumerator1" (`self.HeatLoving`))
              (else
                (goto _label))))
          (:`then_2`
            (if (> (`/Game/Blueprints/BP_Room.Power` _roomreference) 1.0)
              (`/Game/Blueprints/BP_Room.Consume Resource` (`self.RoomReference`) "NewEnumerator2" (`self.Fear`))
              (else
                (goto _label))))
          (:`then_3`
            (if (<= (`self.Health`) 0.0)
              (`/Engine/EditorBlueprintResources/StandardMacros.DoOnce` false
                (:`Completed`
                  (`self.Death`))))))))))

(event `Blink`
  (bind _cubeeyescale (`self.CubeEyeScale`))
  ;[1 1 1] Blinking
  (if (`self.bIsAlive`)
    (bind (_direction _blink_scale) (`Timeline|BlinkTimeline` :!via `PlayFromStart`)
      (:`Update`
        (`SceneComponent.SetRelativeScale3D` (`self.Eye`) (`KismetMathLibrary.MakeVector` _cubeeyescale _cubeeyescale (* _cubeeyescale _blink_scale)))
        (`SceneComponent.SetRelativeScale3D` (`self.Eye2`) (`KismetMathLibrary.MakeVector` _cubeeyescale _cubeeyescale (* _cubeeyescale _blink_scale))))
      (:`Finished`
        (`KismetSystemLibrary.Delay` (`KismetMathLibrary.RandomFloatInRange` 1.0 2.5))
        (`self.Blink`)))))

(event `self.CharacterBody.OnClicked`
  (params (TouchedComponent :type "PrimitiveComponent Object Reference") (ButtonPressed :type "Key Structure"))
  ;[1 1 1] Selection
  (`self.OnClick`))

(event `self.ReceiveTick`
  (params (DeltaSeconds :type "Float (single-precision)"))
  (if (`self.bIsAlive`)
    ;[1 1 1] Change Eye Size in low gravity
    (if (`PrimitiveComponent.IsGravityEnabled` (`self.CharacterBody`))
      (`/Engine/EditorBlueprintResources/StandardMacros.DoOnce` false :!label _label
        (:`Completed`
          (set `self.CubeEyeScale` 0.2)
          (goto _label_2 :!via `Reset`)))
      (else
        (`/Engine/EditorBlueprintResources/StandardMacros.DoOnce` false :!label _label_2
          (:`Completed`
            (set `self.CubeEyeScale` 0.25)
            (goto _label :!via `Reset`)))))))

(event `Select`
  ;[1 1 1] Selection
  (`ActorComponent.Activate` (`self.CharacterSelectionEffect`) true)
  (`self.Change Eye Size` 0.25))

(event `Deselect`
  ;[1 1 1] Selection
  (`ActorComponent.Deactivate` (`self.CharacterSelectionEffect`))
  (`self.Change Eye Size` 0.2))

(event `Death`
  ;[1 1 1] Death
  (`/Engine/EditorBlueprintResources/StandardMacros.DoOnce` false
    (:`Completed`
      (`self.Deselect`)
      (set `self.bIsAlive` false)
      (`MeshComponent.SetScalarParameterValueOnMaterials` (`self.Eye2`) "Highlight" 0.0)
      (`MeshComponent.SetScalarParameterValueOnMaterials` (`self.Eye`) "Highlight" 0.0)
      (bind _asbp_game_instance (cast `/Game/Blueprints/Game/BP_GameInstance` (`GameplayStatics.GetGameInstance`)))
      (`/Engine/EditorBlueprintResources/StandardMacros.DecrementInt` (`/Game/Blueprints/Game/BP_GameInstance.SavedCubes` _asbp_game_instance)))))

(event `Explode In Space`
  ;[1 1 1] Death Explosion Effect
  (`/Engine/EditorBlueprintResources/StandardMacros.DoOnce` false
    (:`Completed`
      (`SceneComponent.SetHiddenInGame` (`self.CharacterBody`) true false)
      (`SceneComponent.SetHiddenInGame` (`self.Eye2`) true false)
      (`SceneComponent.SetHiddenInGame` (`self.Eye`) true false)
      (`SceneComponent.SetHiddenInGame` (`self.CharacterStatusWidget`) true false)
      (`ActorComponent.Activate` (`self.DeathEffect`) true)
      (`self.SetLifeSpan` 2.0))))

(fn `Change Eye Size`
  (params (CubeEyeScale :type "Float (double-precision)"))
  (if (`self.bIsAlive`)
    (bind _output_get (set `self.CubeEyeScale` CubeEyeScale))
    (`SceneComponent.SetRelativeScale3D` (`self.Eye`) (`KismetMathLibrary.Conv_DoubleToVector` _output_get))
    (`SceneComponent.SetRelativeScale3D` (`self.Eye2`) (`KismetMathLibrary.Conv_DoubleToVector` _output_get))))

(fn `Generate Cube Parameters`
  (set `self.Lungs` (`KismetMathLibrary.RandomFloatInRange` 0.8 2.5))
  (set `self.HeatLoving` (`KismetMathLibrary.RandomFloatInRange` 0.8 2.5))
  (set `self.Fear` (`KismetMathLibrary.RandomFloatInRange` 0.8 2.5)))

(fn `OnHover`
  (`MeshComponent.SetScalarParameterValueOnMaterials` (`self.CharacterBody`) "Highlight" 1.2))

(fn `OnHoverEnd`
  (`MeshComponent.SetScalarParameterValueOnMaterials` (`self.CharacterBody`) "Highlight" 1.0))

(fn `Say`
  (params (`Text To Say` :type Text))
  (bind _aswbp_character_status (cast `/Game/Widgets/WBP_CharacterStatus` (`WidgetComponent.GetUserWidgetObject` (`self.CharacterStatusWidget`))))
  (`/Game/Widgets/WBP_CharacterStatus.Say` _aswbp_character_status `Text To Say`))

(fn `UserConstructionScript`)