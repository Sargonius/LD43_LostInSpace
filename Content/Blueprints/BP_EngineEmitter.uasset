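; BP_EngineEmitter handles the sound and Niagara effect of an engine, reacting when its fuel runs out.
; BeginPlay plays the engine sound once at the actor's location, without attaching it or keeping a reference.
; Tick polls GetFuel, and a DoOnce that is never reset deactivates the Niagara component and plays a no-fuel sound when fuel is nearly empty.
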(event `self.ReceiveBeginPlay`
  (`GameplayStatics.PlaySoundAtLocation` "/Game/Sounds/SQ_Engine.SQ_Engine" (`self.K2_GetActorLocation`) (struct) 0.4 1.0 0.0 null null null))

(event `self.ReceiveTick`
  (params (DeltaSeconds :type "Float (single-precision)"))
  (if (<= (`/Game/Blueprints/BPF_LostInSpace.Get Fuel`) 1.0)
    (`/Engine/EditorBlueprintResources/StandardMacros.DoOnce` false
      (:`Completed`
        (`ActorComponent.Deactivate` (`self.NiagaraComponent`))
        (`GameplayStatics.PlaySoundAtLocation` "/Game/Sounds/S_NoFuel.S_NoFuel" (`SceneComponent.K2_GetComponentLocation` (`self.NiagaraComponent`)) (struct) 0.25 1.0 0.0 null null null)))))

(fn `UserConstructionScript`)