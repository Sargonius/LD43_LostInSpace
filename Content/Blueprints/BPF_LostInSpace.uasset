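; Blueprint function library for Lost In Space that provides shared access to fuel.
; Get Fuel returns the Fuel value of the first BP_FuelContainer found in the world, and Consume Fuel subtracts a given amount from it.
; Both look up the container with GetAllActorsOfClass on each call and use index 0, with no empty-array check or clamping.
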(fn `Consume Fuel`
  (params (AmountToConsume :type "Float (double-precision)"))
  (bind _outactors (`GameplayStatics.GetAllActorsOfClass` (`local.__WorldContext`) "/Game/Blueprints/BP_FuelContainer.BP_FuelContainer_C"))
  (bind _output (`|GetArrayItem` _outactors))
  (set `/Game/Blueprints/BP_FuelContainer.Fuel` (- (`/Game/Blueprints/BP_FuelContainer.Fuel` _output) AmountToConsume) _output))

(fn `Get Fuel`
  (returns (Fuel :type "Float (double-precision)"))
  (bind _outactors (`GameplayStatics.GetAllActorsOfClass` (`local.__WorldContext`) "/Game/Blueprints/BP_FuelContainer.BP_FuelContainer_C"))
  (return (`/Game/Blueprints/BP_FuelContainer.Fuel` (`|GetArrayItem` _outactors))))