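; BP_GravityBeam is an actor that traces a gravity beam every tick, affecting characters and rooms it hits.
; A debug-drawn object trace runs from its location to its scaled forward vector, used as an absolute endpoint without location offset.
; A hit BP_Character's Cube loses gravity, simulates physics and is pushed opposite the beam's forward direction.
; A hit BP_Room has its Room collision disabled and its gravity toggled.
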(event `self.ReceiveTick`
  (params (DeltaSeconds :type "Float (single-precision)"))
  (bind _returnvalue (* (`self.GetActorForwardVector`) 10000.0))
  (bind (_outhit _returnvalue_2) (`KismetSystemLibrary.LineTraceSingleForObjects` :`Start` (`self.K2_GetActorLocation`) :`End` _returnvalue :`ObjectTypes` (`|MakeArray` "ObjectTypeQuery3" "ObjectTypeQuery7" :!type "EObjectTypeQuery Enum") :`DrawDebugType` "ForOneFrame"))
  (if _returnvalue_2
    (bind (_bblockinghit _binitialoverlap _time _distance _location _impactpoint _normal _impactnormal _physmat _hitactor) (`GameplayStatics.BreakHitResult` _outhit))
    (bind _asbp_character (cast `/Game/Blueprints/BP_Character` _hitactor)
      (:`then`
        (bind _cube (`/Game/Blueprints/BP_Character.Cube` _asbp_character))
        (`PrimitiveComponent.SetEnableGravity` _cube false)
        (`PrimitiveComponent.SetSimulatePhysics` _cube true)
        (`PrimitiveComponent.AddForceAtLocation` _cube (* _returnvalue -1.0) (`SceneComponent.K2_GetComponentLocation` _cube) "None"))
      (:`CastFailed`
        (bind _asbp_room (cast `/Game/Blueprints/BP_Room` _hitactor))
        (`PrimitiveComponent.SetCollisionEnabled` (`/Game/Blueprints/BP_Room.Room` _asbp_room) "NoCollision")
        (`/Game/Blueprints/BP_Room.Toggle Gravity` _asbp_room)))))

(fn `UserConstructionScript`)